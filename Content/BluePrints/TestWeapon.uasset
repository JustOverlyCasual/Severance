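; TestWeapon is a weapon Blueprint that fires TestProjectile automatically while the trigger is held.
; Pulltrigger passes a DoOnce gate, fires immediately, then starts a looping timer on Fire at an interval derived from RoundsPerSecond.
; Releasetrigger clears that timer and resets the gate.
; Each Fire spawns a projectile at the ProjectileSpawnPoint transform.
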(event Custom|Pulltrigger
  (Utilities|FlowControl|DoOnce false
    (:Completed
      (CallFunction|Fire)
      (Utilities|Time|SetTimerbyFunctionName 0 "Fire" (/ 1.0 (Variables|Default|Getrounds%20per%20second)) true))))

(event Custom|Release%20trigger
  (Utilities|Time|ClearTimerbyFunctionName 0 "fire")
  (Utilities|FlowControl|DoOnce false) ; enters at Reset
)

(event Custom|fire
  (Game|SpawnActorfromClass "/Game/BluePrints/TestProjectile.TestProjectile_C" (Transformation|GetWorldTransform (Variables|Default|GetProjectileSpawnPoint)) "Undefined" 0 0))

(event EventBeginPlay)

(event Collision|EventActorBeginOverlap
  (params (OtherActor :type Actor%20Object%20Reference)))

(event EventTick
  (params (DeltaSeconds :type Float%20%28single-precision%29)))

(fn ConstructionScript)