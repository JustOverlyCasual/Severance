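; Test enemy character that damages the player on overlap and can be killed through AffectHealth.
; Overlapping a PlayerCharacter starts a DamagePlayer timer timed by TimePerSecond, which is cleared when that player's overlap ends.
; AffectHealth runs CalculateHealth and prints health; on death it drops capsule collision with pawns and static world, detaches the controller and destroys the actor after a delay.
; The construction script tints the mesh with EnemyColor through a dynamic material instance.
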(event Custom|DamagePlayer
  (Default|AffectHealth (Variables|Default|GetPlayer) -1e+02))

(event Collision|EventActorBeginOverlap
  (params (OtherActor :type Actor%20Object%20Reference))
  (bind _asplayer_character (Utilities|Casting|CastToPlayerCharacter OtherActor))
  (Variables|Default|SetPlayer _asplayer_character)
  (Utilities|Time|SetTimerbyFunctionName 0 "DamagePlayer" (/ 1.0 (Variables|Default|GetTimePerSecond))))

(event Collision|EventActorEndOverlap
  (params (OtherActor :type Actor%20Object%20Reference))
  (if (== OtherActor (Variables|Default|GetPlayer))
    (Utilities|Time|ClearTimerbyFunctionName 0 "DamagePlayer")))

(event EventAffectHealth
  (params (Delta :type Float%20%28single-precision%29))
  (bind _capsulecomponent (Variables|Default|GetCapsuleComponent))
  (Class|BaseCharacter|CalculateHealth Delta)
  (Development|PrintString (Utilities|String|ToString(Float) (Variables|Default|GetHealth)))
  (if (Variables|Default|GetisDead)
    (Collision|SetCollisionResponsetoChannel _capsulecomponent "ECC_WorldStatic" "ECR_Ignore")
    (Collision|SetCollisionResponsetoChannel _capsulecomponent "ECC_Pawn" "ECR_Ignore")
    (Class|Pawn|DetachfromControllerPendingDestroy)
    (Utilities|FlowControl|Delay 3.0)
    (Actor|DestroyActor)))

(fn ConstructionScript
  (bind _returnvalue (Rendering|Material|CreateDynamicMaterialInstance (Variables|Character|GetMesh) 0 0 "None" :!class /Script/Engine.PrimitiveComponent))
  (bind _output_get (Variables|Default|SetDyna%20Mat _returnvalue))
  (Rendering|Material|SetVectorParameterValue _output_get "BodyColor" (Variables|Default|GetEnemyColor) :!class /Script/Engine.MaterialInstanceDynamic))